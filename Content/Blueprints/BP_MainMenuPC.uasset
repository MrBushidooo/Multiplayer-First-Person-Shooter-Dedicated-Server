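; BP_MainMenuPC is a player controller that brings up the main menu UI.
; On BeginPlay, for the local controller only, it creates WBP_MainMenuWidget, stores a reference and adds it to the viewport.
; It then switches input to UI only with focus on that widget and shows the mouse cursor.
; An unconnected validity check that would re-add the widget never runs.
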(event `self.ReceiveBeginPlay`
  (if (`self.IsLocalController`)
    (bind _returnvalue (`|CreateWidget` "/Game/Widgets/WBP_MainMenuWidget.WBP_MainMenuWidget_C" self))
    (bind _output_get (set `self.MainMenuWidgetRef` _returnvalue))
    (`UserWidget.AddToViewport` _output_get 0)
    (`WidgetBlueprintLibrary.SetInputMode_UIOnlyEx` self _output_get)
    (set `self.bShowMouseCursor` true)))

(fn `UserConstructionScript`)