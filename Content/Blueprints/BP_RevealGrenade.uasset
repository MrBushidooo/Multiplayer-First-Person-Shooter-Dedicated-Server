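; Reveal grenade actor that handles the trail effect and the expanding scan pulse of the grenade.
; The trail activates on BeginPlay, and a separate event stops it.
; PlayPulseVFX plays a radar ping at the given location and writes that location to the MPC_Radius material parameter collection.
; A timeline then animates the collection's Radius parameter to grow the scan, and the actor destroys itself when it finishes.
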(event `self.ReceiveBeginPlay`
  (`ActorComponent.Activate` (`self.TrailVFX`) false))

(event `self.BP_StopTrailVFX`
  (`ActorComponent.Deactivate` (`self.TrailVFX`)))

(event `self.PlayPulseVFX`
  (params (Location :type "Vector Structure"))
  (`GameplayStatics.PlaySoundAtLocation` "/Game/Audio/radar-ping-306440.radar-ping-306440" Location (struct) 1.0 1.0 0.0 null null null null)
  (`KismetMaterialLibrary.SetVectorParameterValue` "/Game/Materials/MPC_Radius.MPC_Radius" "ExplosionLocation" (`KismetMathLibrary.Conv_VectorToLinearColor` Location))
  (bind (_direction _scanradiusgrow) (`Timeline|Timeline` :!via `PlayFromStart`)
    (:`Update`
      (`KismetMaterialLibrary.SetScalarParameterValue` "/Game/Materials/MPC_Radius.MPC_Radius" "Radius" _scanradiusgrow))
    (:`Finished`
      (`self.K2_DestroyActor`))))

(fn `UserConstructionScript`)